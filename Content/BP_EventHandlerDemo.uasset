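; Demo actor that exercises the EventHandlerSubsystem's gameplay-tag-based event broadcasting.
; On BeginPlay it binds to the subsystem's event-fired delegate and broadcasts a simple test event locally.
; Without authority, it also broadcasts a separate test event to the server.
; An auto-generated handler function prints the received event's tag as debug text, leaving the optional payload unused.
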(event EventBeginPlay
  (EventDispatchers|BindEventtoOnEventFiredDelegate (Subsystems|GetEventHandlerSubsystem) (EventDispatchers|CreateEvent :!event BPEventHandlerDemoAutoGenFunc))
  (Class|EventHandlerSubsystem|BroadcastEventLocal (Subsystems|GetEventHandlerSubsystem) "(TagName=\"EventHandler.DemoTest.SimpleEvent\")")
  (Networking|SwitchHasAuthority
    (:Remote
      (Class|EventHandlerSubsystem|BroadcastEventtoServer (Subsystems|GetEventHandlerSubsystem) "(TagName=\"EventHandler.DemoTest.ServerEvent\")"))))

(event Collision|EventActorBeginOverlap
  (params (OtherActor :type Actor%20Object%20Reference)))

(event EventTick
  (params (DeltaSeconds :type Float%20%28single-precision%29)))

(fn ConstructionScript)

(fn BPEventHandlerDemoAutoGenFunc
  (params (EventID :type Gameplay%20Tag%20Structure) (OptionalPayload :type Generic%20Event%20Payload%20Object%20Reference))
  (Development|PrintText (Utilities|Text|FormatText "event received : {x}" (GameplayTags|GetDebugStringfromGameplayTag EventID))))